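; Game mode Blueprint for Toon Tanks that shows the match start and end screens and handles the loss transition.
; StartGame adds the start widget to the viewport, while GameOver adds the end widget with won or lost text.
; After a five-second delay, GameOver stores the current level name and opens the Lose level on a loss.
; A win triggers no level change.
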(event EventBeginPlay)

(event EventTick
  (params (DeltaSeconds :type Float%20%28single-precision%29)))

(event EventStartGame
  (bind _returnvalue (UserInterface|CreateWidget "/Game/Blueprint/Widgets/WB_StartGameWidget.WB_StartGameWidget_C"))
  (UserInterface|Viewport|AddtoViewport _returnvalue 0))

(event EventGameOver
  (params (bWonGame :type Boolean))
  (bind _returnvalue (UserInterface|CreateWidget "/Game/Blueprint/Widgets/WB_EndGameWidget.WB_EndGameWidget_C"))
  (UserInterface|Viewport|AddtoViewport _returnvalue 0)
  (Variables|/Script/UMG.TextBlock|SetText (Variables|/Game/Blueprint/Widgets/WB_EndGameWidget.WB_EndGameWidget_C|GetDisplayText _returnvalue) (select bWonGame "YOU WON" "YOU LOST"))
  (Utilities|FlowControl|Delay 5.0)
  (bind _returnvalue_2 (Game|GetCurrentLevelName true))
  (Variables|Default|SetCurrentLevel _returnvalue_2)
  (if (not bWonGame)
    (Game|OpenLevel(byName) "Lose")))

(fn ConstructionScript)