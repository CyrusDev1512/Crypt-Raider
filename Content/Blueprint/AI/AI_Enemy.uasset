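; AI_Enemy is an enemy AI controller that runs BT_Enemy on possess to drive behavior from perception.
; A successful perception update stores player 0's pawn as the Target blackboard key, whichever actor was sensed.
; Losing the stimulus or failing the pawn cast clears Target immediately.
; Each sighting also sets a looping GiveUpChase timer, but that function is an empty stub.
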(event OnTargetPerceptionUpdated(AIPerception)
  (params (Actor :type Actor%20Object%20Reference) (Stimulus :type AI%20Stimulus%20Structure))
  (bind _blackboard (Variables|Default|GetBlackboard))
  (bind _target (Variables|Default|GetTarget))
  (bind _aspawn (Utilities|Casting|CastToPawn (Game|Player|GetPlayerPawn 0))
    (:then
      (if (.bSuccessfullySensed (Utilities|Struct|BreakAIStimulus Stimulus))
        (AI|Components|Blackboard|SetValueasObject _blackboard _target _aspawn)
        (Development|PrintString "Saw")
        (Utilities|Time|SetTimerbyFunctionName 0 "GiveUpChase" 5.0 true)
        (else
          (AI|Components|Blackboard|SetValueasObject _blackboard _target 0 :!label _label)
          (Development|PrintString "Not Seen"))))
    (:CastFailed
      (goto _label))))

(event EventBeginPlay)

(event EventPossess
  (params (PossessedPawn :type Pawn%20Object%20Reference))
  (AI|RunBehaviorTree "/Game/Blueprint/AI/BT_Enemy.BT_Enemy"))

(fn ConstructionScript)

(fn GiveUpChase)